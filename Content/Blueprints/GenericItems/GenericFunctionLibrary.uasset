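; Generic Blueprint function library with shared helpers for UI widgets and player access.
; TogglePanel either applies a given visibility or flips between Hidden and SelfHitTestInvisible, judging by the passed-in value rather than querying the widget.
; GetPlayer returns player 0's character cast to GenericCharacter.
; AddWidgetToViewport creates and displays a widget of the given class, then sets Game-and-UI input and shows the mouse cursor.
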(fn `AddWidgetToViewport`
  (params (Widget :type "UserWidget Class Reference"))
  (bind _returnvalue (`GameplayStatics.GetPlayerController` null))
  (bind _returnvalue_2 (`|CreateWidget` Widget))
  (`UserWidget.AddToViewport` _returnvalue_2 0)
  (`WidgetBlueprintLibrary.SetInputMode_GameAndUIEx` _returnvalue)
  (set `PlayerController.bShowMouseCursor` true _returnvalue))

(fn `GetPlayer`
  (returns (Character :type "/Game/Blueprints/GenericItems/GenericCharacter Object Reference"))
  (bind _asgeneric_character (cast `/Game/Blueprints/GenericItems/GenericCharacter` (`GameplayStatics.GetPlayerCharacter` null)))
  (return _asgeneric_character))

(fn `TogglePanel`
  (params (Widget :type "Widget Object Reference") (Visibility :type "ESlateVisibility Enum") (SetVisibility :type Boolean))
  (locals (WidgetLocal :type "Widget Object Reference") (VisbilityLocal :type "ESlateVisibility Enum") (SetLocal :type Boolean))
  (set `local.WidgetLocal` Widget)
  (set `local.VisbilityLocal` Visibility)
  (bind _output_get (set `local.SetLocal` SetVisibility))
  (if _output_get
    (`Widget.SetVisibility` (`local.WidgetLocal`) (`local.VisbilityLocal`)) ; Setting to Passed in Visibility
    (else
      (switch `ESlateVisibility` (`local.VisbilityLocal`) ; Toggling based on Current Visibility
        (:`Collapsed`
          (`Widget.SetVisibility` (`local.WidgetLocal`) "SelfHitTestInvisible" :!label _label) ; Toggling to Hidden
        )
        (:`Hidden`
          (goto _label))
        (:`SelfHitTestInvisible`
          (`Widget.SetVisibility` (`local.WidgetLocal`) "Hidden") ; Toggling to Hidden
        )))))